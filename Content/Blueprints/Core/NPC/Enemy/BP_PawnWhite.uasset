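; BP_PawnWhite is an enemy NPC Blueprint that gives its static mesh a black outline on BeginPlay.
; CreateOutline spawns an unattached duplicate mesh component at the original's world transform, using a dynamic instance of M_OutlineClean_Inst for color and scale.
; The HasOutline flag prevents duplicate outlines.
; DestroyOutline removes the component and clears the flag, but is not called within this Blueprint.
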(event EventBeginPlay
  (Variables|Default|SetHasOutline false)
  (Variables|Default|SetAtualMesh (Variables|/Script/Engine.StaticMeshComponent|GetStaticMesh (Variables|Default|GetStaticMesh)))
  (Variables|Default|SetColor "(R=0.000000,G=0.000000,B=0.000000,A=1.000000)")
  (Variables|Default|SetScale 2.0)
  (CallFunction|CreateOutline))

(event Collision|EventActorBeginOverlap
  (params (OtherActor :type Actor%20Object%20Reference)))

(event EventTick
  (params (DeltaSeconds :type Float%20%28single-precision%29)))

(fn ConstructionScript)

(fn CreateOutline
  (if (not (Variables|Default|GetHasOutline))
    (bind _returnvalue (AddComponent|AddStaticMeshComponent true (Transformation|GetWorldTransform (Variables|Default|GetStaticMesh))))
    (bind _output_get (Variables|Default|SetMeshComp _returnvalue))
    (Components|StaticMesh|SetStaticMesh _output_get (Variables|Default|GetAtualMesh))
    (bind _returnvalue_2 (Rendering|Material|CreateDynamicMaterialInstance (Variables|Default|GetMeshComp) 0 "/Game/Art/Materials/Outline/M_OutlineClean_Inst.M_OutlineClean_Inst" "None" :!class /Script/Engine.PrimitiveComponent))
    (Rendering|Material|SetVectorParameterValue _returnvalue_2 "color" (Variables|Default|GetColor) :!class /Script/Engine.MaterialInstanceDynamic)
    (Rendering|Material|SetScalarParameterValue _returnvalue_2 "Scale" (Variables|Default|GetScale) :!class /Script/Engine.MaterialInstanceDynamic)
    (Variables|Default|SetHasOutline true)))

(fn DestroyOutline
  (bind _meshcomp (Variables|Default|GetMeshComp))
  (Utilities|IsValid _meshcomp
    (:Is%20Valid
      (Components|DestroyComponent _meshcomp)
      (Variables|Default|SetHasOutline false))))
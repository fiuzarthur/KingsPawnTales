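; BP_GridModifier is a grid marker actor that displays a tile Type in the editor and is hidden in game.
; Its construction script applies a fixed shape's mesh and flat material from GetShapeData, then sets a filled look colored by Type (None, Normal, Obstacle, River or upgrade variants).
; The mesh overlaps a custom trace channel, and the event graph holds no logic.
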(event EventBeginPlay)

(event Collision|EventActorBeginOverlap
  (params (OtherActor :type Actor%20Object%20Reference)))

(event EventTick
  (params (DeltaSeconds :type Float%20%28single-precision%29)))

(fn ConstructionScript
  (bind _data (CallFunction|GetShapeData "NewEnumerator1"))
  (bind _staticmesh (Variables|Default|GetStaticMesh))
  (bind _staticmesh_2 (Variables|Default|GetStaticMesh))
  (Components|StaticMesh|SetStaticMesh _staticmesh (.mesh _data))
  (Rendering|Material|SetMaterial _staticmesh_2 0 (.flatmat _data))
  (Rendering|Material|SetVectorParameterValueonMaterials _staticmesh "Color" (Math|Conversions|ToVector(LinearColor) (Utilities|Select :Index (Variables|Default|GetType) :NewEnumerator0 "" :NewEnumerator1 "(R=1.000000,G=1.000000,B=1.000000,A=1.000000)" :NewEnumerator2 "(R=0.942708,G=0.039280,B=0.039280,A=1.000000)" :NewEnumerator3 "(R=0.160463,G=0.311570,B=0.687500,A=1.000000)" :NewEnumerator4 "(R=0.786458,G=0.143365,B=0.702052,A=1.000000)" :NewEnumerator5 "(R=0.885417,G=0.806215,B=0.193685,A=1.000000)")))
  (Rendering|Material|SetScalarParameterValueonMaterials _staticmesh_2 "IsFilled" 1.0)
  (Collision|SetCollisionResponsetoChannel (Variables|Default|GetStaticMesh) "ECC_GameTraceChannel1" "ECR_Overlap")
  (Rendering|SetActorHiddenInGame true))
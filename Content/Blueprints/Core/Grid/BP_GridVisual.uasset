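; BP_GridVisual is the actor that renders the grid's tiles through a child BP_GridMeshInst instanced-mesh actor, with ticking disabled.
; InitializeGridVisual stores the grid, sets up the instancer with the flat mesh and material from the "Square" shape data row, then places itself at the world origin raised by a ground offset.
; Tile updates remove and re-add that tile's instance with its transform and states, while destroying the visual clears all instances.
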(event EventBeginPlay
  (Actor|Tick|SetActorTickEnabled false))

(event Collision|EventActorBeginOverlap
  (params (OtherActor :type Actor%20Object%20Reference)))

(event EventTick
  (params (DeltaSeconds :type Float%20%28single-precision%29)))

(fn ConstructionScript)

(fn InitializeGridVisual
  (params (Grid :type BP%20Grid%20Object%20Reference))
  (Variables|Default|SetGrid Grid)
  (Variables|Default|SetGrid%20Mesh%20Inst (.AsBP%20Grid%20Mesh%20Inst (Utilities|Casting|CastToBP_GridMeshInst (Variables|/Script/Engine.ChildActorComponent|GetChildActor (Variables|Default|GetChildActor_GridMeshInst)))))
  (bind _returnvalue (Utilities|GetDataTableRow "/Game/Blueprints/Core/Grid/GridShapes/DT_GridShapeData.DT_GridShapeData" "Square")
    (:then
      (Default|InitializeGridMeshInst :self (Variables|Default|GetGrid%20Mesh%20Inst) :NewMesh (.FlatMesh (Utilities|Struct|BreakS_GridShapeData _returnvalue)) :Material (.FlatMat (Utilities|Struct|BreakS_GridShapeData _returnvalue)) :Colision "QueryOnly")
      (Transformation|SetActorLocation "0, 0, 0" false false) ; enterr Grid In World
      (CallFunction|SetOffsetfromGround))))

(fn SetOffsetfromGround
  (bind _returnvalue (Transformation|GetActorLocation))
  (Transformation|SetActorLocation (Math|Vector|MakeVector (.x _returnvalue) (.y _returnvalue) (Variables|Default|GetOffsetFromGround)) false false))

(fn DestroyGridVisual
  (Utilities|IsValid (Variables|Default|GetGrid%20Mesh%20Inst)
    (:Is%20Valid
      (Default|ClearInstances (Variables|Default|GetGrid%20Mesh%20Inst)))))

(fn UpdateTilesVisual
  (params (Data :type S%20Tile%20Data%20Structure))
  (Default|RemoveInstance (Variables|Default|GetGrid%20Mesh%20Inst) (.index Data))
  (Default|AddInstance (Variables|Default|GetGrid%20Mesh%20Inst) (.transform Data) (.index Data) (.states Data)))
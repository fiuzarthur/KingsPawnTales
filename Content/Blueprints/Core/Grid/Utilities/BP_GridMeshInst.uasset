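; Grid visual actor that draws tiles as instances of one InstancedStaticMesh, with mesh, material, color and collision set on initialization.
; An InstanceIndexes array maps grid indices to instances, so re-adding a tile replaces its old instance.
; Tile states resolve by priority (Selected, Hovered, IsNeighbor) to a color and filled flag, written as per-instance custom data.
; Tick is disabled at BeginPlay.
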(event EventBeginPlay
  (Actor|Tick|SetActorTickEnabled false))

(event Collision|EventActorBeginOverlap
  (params (OtherActor :type Actor%20Object%20Reference)))

(event EventTick
  (params (DeltaSeconds :type Float%20%28single-precision%29)))

(fn ConstructionScript)

(fn AddInstance
  (params (InstanceTransform :type Transform%20%28by%20ref%29) (Index :type Int%20Point%20Structure%20%28by%20ref%29) (State :type Array%20of%20E_TileState%20Enums :default "NewEnumerator0"))
  (bind _instancedstaticmesh (Variables|Default|GetInstancedStaticMesh))
  (CallFunction|RemoveInstance Index)
  (Components|InstancedStaticMesh|AddInstance (Variables|Default|GetInstancedStaticMesh) InstanceTransform)
  (bind _returnvalue (Utilities|Array|Add (Variables|Default|GetInstanceIndexes) Index))
  (LocalVariables|SetI _returnvalue)
  (bind (_color _isfilled) (CallFunction|GetColorfromStates State))
  (Components|InstancedStaticMesh|SetCustomDataValue _instancedstaticmesh (LocalVariables|GetI) 0 (.R (Math|Color|BreakColor _color)) false)
  (Components|InstancedStaticMesh|SetCustomDataValue _instancedstaticmesh (LocalVariables|GetI) 1 (.G (Math|Color|BreakColor _color)) false)
  (Components|InstancedStaticMesh|SetCustomDataValue _instancedstaticmesh (LocalVariables|GetI) 2 (.B (Math|Color|BreakColor _color)) false)
  (Components|InstancedStaticMesh|SetCustomDataValue _instancedstaticmesh (LocalVariables|GetI) 3 _isfilled false))

(fn RemoveInstance
  (params (ItemToFind :type Int%20Point%20Structure%20%28by%20ref%29))
  (bind _instanceindexes (Variables|Default|GetInstanceIndexes))
  (if (Utilities|Array|ContainsItem :TargetArray _instanceindexes)
    (Class|InstancedStaticMeshComponent|RemoveInstance (Variables|Default|GetInstancedStaticMesh) (Utilities|Array|FindItem _instanceindexes ItemToFind))
    (Utilities|Array|RemoveItem (Variables|Default|GetInstanceIndexes) ItemToFind)))

(fn ClearInstances
  (Components|InstancedStaticMesh|ClearInstances (Variables|Default|GetInstancedStaticMesh))
  (Utilities|Array|Clear (Variables|Default|GetInstanceIndexes)))

(fn InitializeGridMeshInst
  (params (NewMesh :type Static%20Mesh%20Object%20Reference) (Material :type Material%20Interface%20Object%20Reference) (Color :type Linear%20Color%20Structure) (Colision :type ECollisionEnabled%20Enum :default "NoCollision"))
  (bind _instancedstaticmesh (Variables|Default|GetInstancedStaticMesh))
  (Components|StaticMesh|SetStaticMesh _instancedstaticmesh NewMesh)
  (Rendering|Material|SetMaterial _instancedstaticmesh 0 Material)
  (Rendering|Material|SetVectorParameterValueonMaterials _instancedstaticmesh "Color" (Math|Conversions|ToVector(LinearColor) Color))
  (Collision|SetCollisionEnabled _instancedstaticmesh Colision))

(fn GetColorfromStates
  (params (States :type Array%20of%20E_TileState%20Enums :default "NewEnumerator0"))
  (if (== (Utilities|Array|Length States) 0)
    (return "" 0.0)
    (else
      (for _array_element (Utilities|Array|MakeArray "NewEnumerator2" "NewEnumerator1" "NewEnumerator3")
        (if (Utilities|Array|ContainsItem States _array_element)
          (return (Utilities|Select :Index _array_element :NewEnumerator0 "" :NewEnumerator2 "(R=0.994792,G=0.497572,B=0.487033,A=1.000000)" :NewEnumerator1 "(R=0.968750,G=0.925926,B=0.575195,A=1.000000)" :NewEnumerator3 "(R=1.000000,G=0.255208,B=0.813802,A=1.000000)") 1.0)))
      (return "" 0.0))))
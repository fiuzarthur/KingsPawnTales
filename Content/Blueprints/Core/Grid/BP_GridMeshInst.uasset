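; BP_GridMeshInst is a grid actor that draws meshes through one InstancedStaticMesh component, with actor tick turned off at BeginPlay.
; An init function sets its mesh, material, Color parameter and collision.
; InstanceIndexes parallels the instance order, so an external index's array position locates the instance to remove.
; Adding an index first removes its existing instance, and clearing empties both component and array.
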(event EventBeginPlay
  (Actor|Tick|SetActorTickEnabled false))

(event Collision|EventActorBeginOverlap
  (params (OtherActor :type Actor%20Object%20Reference)))

(event EventTick
  (params (DeltaSeconds :type Float%20%28single-precision%29)))

(fn ConstructionScript)

(fn AddInstance
  (params (InstanceTransform :type Transform%20%28by%20ref%29) (Index :type Int%20Point%20Structure%20%28by%20ref%29))
  (CallFunction|RemoveInstance Index)
  (Components|InstancedStaticMesh|AddInstance (Variables|Default|GetInstancedStaticMesh) InstanceTransform)
  (Utilities|Array|Add (Variables|Default|GetInstanceIndexes) Index))

(fn RemoveInstance
  (params (ItemToFind :type Int%20Point%20Structure%20%28by%20ref%29))
  (bind _instanceindexes (Variables|Default|GetInstanceIndexes))
  (if (Utilities|Array|ContainsItem :TargetArray _instanceindexes)
    (Class|InstancedStaticMeshComponent|RemoveInstance (Variables|Default|GetInstancedStaticMesh) (Utilities|Array|FindItem _instanceindexes ItemToFind))
    (Utilities|Array|RemoveItem (Variables|Default|GetInstanceIndexes) ItemToFind)))

(fn ClearInstances
  (Components|InstancedStaticMesh|ClearInstances (Variables|Default|GetInstancedStaticMesh))
  (Utilities|Array|Clear (Variables|Default|GetInstanceIndexes)))

(fn InitializeGridMeshInst
  (params (NewMesh :type Static%20Mesh%20Object%20Reference) (Material :type Material%20Interface%20Object%20Reference) (Color :type Linear%20Color%20Structure) (Colision :type ECollisionEnabled%20Enum :default "NoCollision"))
  (bind _instancedstaticmesh (Variables|Default|GetInstancedStaticMesh))
  (Components|StaticMesh|SetStaticMesh _instancedstaticmesh NewMesh)
  (Rendering|Material|SetMaterial _instancedstaticmesh 0 Material)
  (Rendering|Material|SetVectorParameterValueonMaterials _instancedstaticmesh "Color" (Math|Conversions|ToVector(LinearColor) Color))
  (Collision|SetCollisionEnabled _instancedstaticmesh Colision))
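; GM_Base is a game mode Blueprint that keeps turn state for what appears to be a turn-based game with controllable pieces.
; ResetAllTurns sets YourTurn to true on the current game mode and calls ResetTurn on every BPC_PieceControllable actor in the world.
; TurnPass increments TurnCount and ResetGame sets it back to one, while the event graph and construction script stay empty.
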(event EventBeginPlay)

(event EventTick
  (params (DeltaSeconds :type Float%20%28single-precision%29)))

(fn ConstructionScript)

(fn ResetAllTurns
  (bind _asgm_base (Utilities|Casting|CastToGM_Base (Game|GetGameMode)))
  (Variables|GM_Base_C|SetYourTurn _asgm_base true)
  (bind _outactors (Actor|GetAllActorsOfClass "/Game/Blueprints/Core/Player/Pieces/BPC_PieceControllable.BPC_PieceControllable_C"))
  (for _array_element _outactors
    (Default|ResetTurn _array_element)))

(fn TurnPass
  (Math|Integer|IncrementInt (Variables|Default|GetTurnCount)))

(fn ResetGame
  (Variables|Default|SetTurnCount 1))
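; Player pawn for a grid-based chess game, combining an overhead-style spring-arm camera with mouse-driven piece selection and movement.
; Input sets desired zoom, location and stepped yaw, which Tick interpolates toward; pan speed scales with arm length.
; Left click traces under the cursor to select a BP_Chess piece, or asks the saved piece to validate and smoothly move to the BP_Grid tile, then deselects.
; Right click prints the hovered tile index.
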(event EventTick
  (params (DeltaSeconds :type Float%20%28single-precision%29))
  ;[0 0 0] Tick
  (Utilities|FlowControl|Sequence
    (:then_0
      ;;[0.1745 0.1751 0.1771] Set Zoom Smoothly
      (Variables|/Script/Engine.SpringArmComponent|SetTargetArmLength (Variables|Default|GetSpringArm) (Math|Interpolation|FInterpTo (Variables|/Script/Engine.SpringArmComponent|GetTargetArmLength (Variables|Default|GetSpringArm)) (Variables|Default|GetZoomDesired) DeltaSeconds (Variables|Default|GetInterp%20Speed%20Zoom)))
      ;;[0.1745 0.1751 0.1771] Set Location Smoothly
      (Transformation|SetActorLocation (Math|Interpolation|VInterpTo (Transformation|GetActorLocation) (Variables|Default|GetLocationDesired) DeltaSeconds (Variables|Default|GetInterp%20Speed%20Location)) false false)
      ;;[0.1745 0.1751 0.1771] Set Rotation Smoothly
      (Transformation|SetActorRotation (Math|Interpolation|RInterpTo (Transformation|GetActorRotation) (Variables|Default|GetRotation%20Desired) DeltaSeconds (Variables|Default|GetInterp%20Speed%20Rotation))))))

(event EventBeginPlay
  ;[0 0 0] Begin Play
  ;;[0.1745 0.1751 0.1771] Set Variable Default Vallues
  (Variables|Default|SetLocationDesired (Transformation|GetActorLocation))
  (Variables|Default|SetZoomDesired (Variables|/Script/Engine.SpringArmComponent|GetTargetArmLength (Variables|Default|GetSpringArm)))
  (Variables|Default|SetRotation%20Desired (Transformation|GetActorRotation))
  (bind _returnvalue (Actor|GetActorOfClass "/Game/Blueprints/Core/Grid/BP_Grid.BP_Grid_C"))
  (Variables|Default|SetGrid _returnvalue))

(event Input|ActionEvents|InputActionRotate_Left
  (params (Key :type Key%20Structure :default "None"))
  ;[1 0.8537 0.1051] Inputs
  ;;[0 0.4776 1] Left Rotation
  (:Pressed
    (Variables|Default|SetRotation%20Desired (Math|Rotator|CombineRotators (Variables|Default|GetRotation%20Desired) (Math|Rotator|MakeRotator 0.0 0.0 (Variables|Default|GetRotationSpeed))))))

(event Input|ActionEvents|InputActionRotate_Right
  (params (Key :type Key%20Structure :default "None"))
  ;[1 0.8537 0.1051] Inputs
  ;;[0 0.4776 1] Right Rotation
  (:Pressed
    (Variables|Default|SetRotation%20Desired (Math|Rotator|CombineRotators (Variables|Default|GetRotation%20Desired) (Math|Rotator|MakeRotator 0.0 0.0 (* (Variables|Default|GetRotationSpeed) -1.0))))))

(event Input|ActionEvents|InputActionLeftMouseButton
  (params (Key :type Key%20Structure :default "None"))
  (bind _returnvalue (Game|GetPlayerController 0))
  (bind (_worldlocation _worlddirection) (Game|Player|ConvertMouseLocationToWorldSpace _returnvalue))
  (:Pressed
    ;[1 0.7565 0] Find Piece On Click
    (bind (_outhit _returnvalue_2) (Collision|LineTraceByChannel _worldlocation (+ _worldlocation (* _worlddirection 1e+04)) "TraceTypeQuery5" false 0 "ForDuration"))
    (if _returnvalue_2
      ;[0 0 0] Get Piece Clicked Select It and Save It
      (bind _asbp_chess (Utilities|Casting|CastToBP_Chess (.HitActor (Collision|BreakHitResult _outhit))))
      (bind _outactors (Actor|GetAllActorsOfClass "/Game/Blueprints/Core/Player/Pieces/BP_Chess.BP_Chess_C"))
      (Default|UnSelect _outactors)
      (Default|Select _asbp_chess)
      (Variables|Default|SetSavedPiece _asbp_chess)
      (Variables|Default|SetHasActor true)
      (else
        (if (Variables|Default|GetHasActor)
          (bind _index (Default|GetTileIndexUnderCursor (Variables|Default|GetGrid)))
          (bind _asbp_chess_2 (Utilities|Casting|CastToBP_Chess (Variables|Default|GetSavedPiece)))
          (bind _found (Default|CheckMovableSpace _asbp_chess_2 _index))
          (if _found
            (if (.ReturnValue (Utilities|Map|Find (Variables|/Game/Blueprints/Core/Grid/BP_Grid.BP_Grid_C|GetGridTiles (Variables|Default|GetGrid)) _index))
              (Default|SmoothMovement _asbp_chess_2 (.location (.Transform (Utilities|Struct|BreakS_TileData (.Value (Utilities|Map|Find (Variables|/Game/Blueprints/Core/Grid/BP_Grid.BP_Grid_C|GetGridTiles (Variables|Default|GetGrid)) _index)))))))))
        (bind _outactors_2 (Actor|GetAllActorsOfClass "/Game/Blueprints/Core/Player/Pieces/BP_Chess.BP_Chess_C"))
        (Default|UnSelect _outactors_2)
        (Variables|Default|SetSavedPiece 0)
        (Variables|Default|SetHasActor false)))))

(event Input|ActionEvents|InputActionRightMouseButton
  (params (Key :type Key%20Structure :default "None"))
  (:Pressed
    (bind _index (Default|GetTileIndexUnderCursor (Variables|Default|GetGrid)))
    (Development|PrintString (Utilities|String|ToString(Integer) _index))))

(event Input|AxisEvents|InputAxisZoom_Input
  (params (AxisValue :type Float%20%28single-precision%29))
  ;[1 0.8537 0.1051] Inputs
  ;;[0 0.4776 1] Zoom
  (Variables|Default|SetZoomDesired (Math|Float|Clamp(Float) (- (Variables|Default|GetZoomDesired) (* AxisValue (Variables|Default|GetZoomSpeed))) (Variables|Default|GetZoomMin) (Variables|Default|GetZoomMax))))

(event Input|AxisEvents|InputAxisForward_Input
  (params (AxisValue :type Float%20%28single-precision%29))
  ;[1 0.8537 0.1051] Inputs
  ;;[0 0.4776 1] Forward Movement
  (Variables|Default|SetLocationDesired (+ (Variables|Default|GetLocationDesired) (* (Transformation|GetActorForwardVector) (* (* AxisValue (/ (Variables|Default|GetLocationSpeed) 1e+02)) (Variables|/Script/Engine.SpringArmComponent|GetTargetArmLength (Variables|Default|GetSpringArm)))))))

(event Input|AxisEvents|InputAxisRight_Input
  (params (AxisValue :type Float%20%28single-precision%29))
  ;[1 0.8537 0.1051] Inputs
  ;;[0 0.4776 1] Right Movement
  (Variables|Default|SetLocationDesired (+ (Variables|Default|GetLocationDesired) (* (Transformation|GetActorRightVector) (* (* AxisValue (/ (Variables|Default|GetLocationSpeed) 1e+02)) (Variables|/Script/Engine.SpringArmComponent|GetTargetArmLength (Variables|Default|GetSpringArm)))))))

(fn ConstructionScript)

(fn ResetSpeed
  (Variables|Default|SetLocationSpeed 2.0))
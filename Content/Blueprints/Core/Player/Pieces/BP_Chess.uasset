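; Chess piece actor that snaps to its BP_Grid tile, tracks selection and computes the tiles it can move to.
; King, pawn, rook and bishop functions combine straight and diagonal probes through the grid's location check into DisponibleSpaces, which CheckMovableSpace queries.
; SmoothMovement lerps piece and outline along a timeline, then deselects.
; The outline is a duplicate mesh component with a dynamic material, rebuilt on selection changes to alter color and thickness.
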(event Custom|SmoothMovement
  (params (FinalPoint :type Vector))
  (bind _meshcomp (Variables|Default|GetMeshComp))
  ;[0 0 0] Gradualy Move the piece
  (if (Variables|Default|GetCanmove)
    (Variables|Movement|SetDestination FinalPoint)
    (Variables|Movement|SetStart (Transformation|GetActorLocation))
    (bind _alpha (Timeline|Timeline1 PlayFromStart) ; Move Speed
      (:Update
        (Variables|Default|SetCanmove false)
        (Transformation|SetActorLocation (Math|Vector|Lerp(Vector) (Variables|Movement|GetStart) (Variables|Movement|GetDestination) _alpha) false false) ; Set Base Location
        (Utilities|IsValid _meshcomp
          (:Is%20Valid
            (Transformation|SetWorldLocation _meshcomp (Math|Vector|Lerp(Vector) (Variables|Movement|GetStart) (Variables|Movement|GetDestination) _alpha) false false) ; Move Outline Along
          )))
      (:Finished
        (CallFunction|UnSelect)
        (Variables|Default|SetCanmove true)))))

(event EventBeginPlay
  ;[0 0 0] Begin Play Set Variables
  (Variables|Outline|SetHasOutline false)
  (Variables|Default|SetAtualMesh (Variables|/Script/Engine.StaticMeshComponent|GetStaticMesh (Variables|Default|GetMesh)))
  (bind _output_get (Variables|Outline|SetColor "(R=1.000000,G=1.000000,B=1.000000,A=1.000000)"))
  (Variables|Default|SetOGColor _output_get)
  (bind _output_get_2 (Variables|Outline|SetScale 1.0))
  (Variables|Default|SetOGScale _output_get_2)
  (bind _returnvalue (Actor|GetActorOfClass "/Game/Blueprints/Core/Grid/BP_Grid.BP_Grid_C"))
  (Variables|Default|SetGrid _returnvalue)
  ;;[1 1 1] Fix
  (Utilities|FlowControl|Delay 0.2)
  (CallFunction|SetBaseLocation)
  (CallFunction|CreateOutline))

(fn ConstructionScript)

(fn CreateOutline
  ;[0 0 0] If Dont Have Outline in the Piece Create One
  (if (not (Variables|Outline|GetHasOutline))
    (bind _returnvalue (AddComponent|AddStaticMeshComponent true (Transformation|GetWorldTransform (Variables|Default|GetMesh))))
    (bind _output_get (Variables|Default|SetMeshComp _returnvalue))
    (Components|StaticMesh|SetStaticMesh _output_get (Variables|Default|GetAtualMesh)) ; Outline Shape
    (bind _returnvalue_2 (Rendering|Material|CreateDynamicMaterialInstance (Variables|Default|GetMeshComp) 0 "/Game/Art/Materials/Outline/OutlineNAMÂO/M_OutlineClean_White.M_OutlineClean_White" "None" :!class /Script/Engine.PrimitiveComponent)) ; Outline Material
    (Rendering|Material|SetVectorParameterValue _returnvalue_2 "color" (Variables|Outline|GetColor) :!class /Script/Engine.MaterialInstanceDynamic) ; Outline Color
    (Rendering|Material|SetScalarParameterValue _returnvalue_2 "Scale" (Variables|Outline|GetScale) :!class /Script/Engine.MaterialInstanceDynamic) ; Outline Thickness
    (Variables|Outline|SetHasOutline true)))

(fn DestroyOutline
  (bind _meshcomp (Variables|Default|GetMeshComp))
  (Utilities|IsValid _meshcomp
    (:Is%20Valid
      (Components|DestroyComponent _meshcomp)
      (Variables|Outline|SetHasOutline false))))

(fn Select
  ;[0.6798 0.1602 1] Save Piece And Change Its Outline
  (Variables|Default|SetSelected true)
  (Variables|Outline|SetColor "(R=1.000000,G=0.887345,B=0.000000,A=1.000000)")
  (Variables|Outline|SetScale (* (Variables|Default|GetOGScale) 3.0))
  (CallFunction|DestroyOutline)
  (CallFunction|CreateOutline)
  (CallFunction|ClearSpaces))

(fn UnSelect
  (Variables|Default|SetSelected false)
  (Variables|Outline|SetColor (Variables|Default|GetOGColor))
  (Variables|Outline|SetScale (Variables|Default|GetOGScale))
  (CallFunction|DestroyOutline)
  (CallFunction|CreateOutline))

(fn SetBaseLocation
  (bind _returnvalue (Transformation|GetActorLocation))
  (bind _height (Variables|Movement|GetHeight))
  ;[0.5168 0.09321 1] Snap Piece To Grid Center
  (bind (_returnvalue_2 _index) (Default|CheckPieceLocation (Variables|Default|GetGrid) (+ _returnvalue _height) (- _returnvalue _height)))
  (if _returnvalue_2
    (if (.ReturnValue (Utilities|Map|Find (Variables|/Game/Blueprints/Core/Grid/BP_Grid.BP_Grid_C|GetGridTiles (Variables|Default|GetGrid)) _index))
      (Transformation|SetActorLocation (.location (.Transform (Utilities|Struct|BreakS_TileData (.Value (Utilities|Map|Find (Variables|/Game/Blueprints/Core/Grid/BP_Grid.BP_Grid_C|GetGridTiles (Variables|Default|GetGrid)) _index))))) false false))))

(fn CheckFrontBackSpace
  (params (Reach :type Integer) (TileSizeX :type Float%20%28single-precision%29))
  (bind _height (Variables|Movement|GetHeight))
  (for _index (range 0 Reach)
    (LocalVariables|SetTileDist (+ (LocalVariables|GetTileDist) TileSizeX))
    (bind (_returnvalue _index_2) (Default|CheckPieceLocation (Variables|Default|GetGrid) (+ (+ (Transformation|GetWorldLocation (Variables|Default|GetMesh)) (Math|Vector|MakeVector (LocalVariables|GetTileDist) 0.0 0.0)) _height) (- (+ (Transformation|GetWorldLocation (Variables|Default|GetMesh)) (Math|Vector|MakeVector (LocalVariables|GetTileDist) 0.0 0.0)) _height)))
    (if _returnvalue
      (Utilities|Array|Add (Variables|Default|GetDisponibleSpaces) _index_2))))

(fn CheckLeftRightSpaces
  (params (Reach :type Integer) (TileSizeY :type Float%20%28single-precision%29))
  (bind _height (Variables|Movement|GetHeight))
  (for _index (range 0 Reach)
    (LocalVariables|SetTileDist (+ (LocalVariables|GetTileDist) TileSizeY))
    (bind (_returnvalue _index_2) (Default|CheckPieceLocation (Variables|Default|GetGrid) (+ (+ (Transformation|GetWorldLocation (Variables|Default|GetMesh)) (Math|Vector|MakeVector 0.0 (LocalVariables|GetTileDist) 0.0)) _height) (- (+ (Transformation|GetWorldLocation (Variables|Default|GetMesh)) (Math|Vector|MakeVector 0.0 (LocalVariables|GetTileDist) 0.0)) _height)))
    (if _returnvalue
      (Utilities|Array|Add (Variables|Default|GetDisponibleSpaces) _index_2))))

(fn ClearSpaces
  (Utilities|Array|Clear (Variables|Default|GetDisponibleSpaces)))

(fn CheckDiagonal+X
  (params (Reach :type Integer) (YDir :type Float%20%28single-precision%29))
  (bind _height (Variables|Movement|GetHeight))
  (for _index (range 0 Reach)
    (LocalVariables|SetXDist (+ (LocalVariables|GetXDist) (.x (Variables|Default|GetTileSize))))
    (LocalVariables|SetTileDist (+ (LocalVariables|GetTileDist) YDir))
    (bind (_returnvalue _index_2) (Default|CheckPieceLocation (Variables|Default|GetGrid) (+ (+ (Transformation|GetWorldLocation (Variables|Default|GetMesh)) (Math|Vector|MakeVector (LocalVariables|GetXDist) (LocalVariables|GetTileDist) 0.0)) _height) (- (+ (Transformation|GetWorldLocation (Variables|Default|GetMesh)) (Math|Vector|MakeVector (LocalVariables|GetXDist) (LocalVariables|GetTileDist) 0.0)) _height)))
    (if _returnvalue
      (Utilities|Array|Add (Variables|Default|GetDisponibleSpaces) _index_2))))

(fn CheckDiagonal-X
  (params (Reach :type Integer) (Ydir :type Float%20%28single-precision%29))
  (bind _height (Variables|Movement|GetHeight))
  (for _index (range 0 Reach)
    (LocalVariables|SetXDist (- (LocalVariables|GetXDist) (.x (Variables|Default|GetTileSize))))
    (LocalVariables|SetTileDist (+ (LocalVariables|GetTileDist) Ydir))
    (bind (_returnvalue _index_2) (Default|CheckPieceLocation (Variables|Default|GetGrid) (+ (+ (Transformation|GetWorldLocation (Variables|Default|GetMesh)) (Math|Vector|MakeVector (LocalVariables|GetXDist) (LocalVariables|GetTileDist) 0.0)) _height) (- (+ (Transformation|GetWorldLocation (Variables|Default|GetMesh)) (Math|Vector|MakeVector (LocalVariables|GetXDist) (LocalVariables|GetTileDist) 0.0)) _height)))
    (if _returnvalue
      (Utilities|Array|Add (Variables|Default|GetDisponibleSpaces) _index_2))))

(fn KingMovement
  ;[1 1 1] FrontAndBackTiles
  (MovementType|CheckFrontBackSpace (Variables|Default|GetReach) (.x (Variables|Default|GetTileSize)))
  (MovementType|CheckFrontBackSpace (Variables|Default|GetReach) (* (.x (Variables|Default|GetTileSize)) -1.0))
  ;[1 1 1] Left And Right Tiles
  (MovementType|CheckLeftRightSpaces (Variables|Default|GetReach) (.y (Variables|Default|GetTileSize)))
  (MovementType|CheckLeftRightSpaces (Variables|Default|GetReach) (* (.y (Variables|Default|GetTileSize)) -1.0))
  ;[1 1 1] Front Diagonal Tiles
  (MovementType|CheckDiagonal+X (Variables|Default|GetReachDiag) (.y (Variables|Default|GetTileSize)))
  (MovementType|CheckDiagonal+X (Variables|Default|GetReachDiag) (* (.y (Variables|Default|GetTileSize)) -1.0))
  ;[1 1 1] Back Diagonal Tiles
  (MovementType|CheckDiagonal-X (Variables|Default|GetReachDiag) (.y (Variables|Default|GetTileSize)))
  (MovementType|CheckDiagonal-X (Variables|Default|GetReachDiag) (* (.y (Variables|Default|GetTileSize)) -1.0)))

(fn CheckMovableSpace
  (params (Index :type Int%20Point%20Structure))
  (bind _disponiblespaces (Variables|Default|GetDisponibleSpaces))
  (bind _returnvalue (Utilities|Array|FindItem _disponiblespaces Index))
  (if (!= _returnvalue -1)
    (return true (Utilities|Array|Get(acopy) (Variables|Default|GetDisponibleSpaces) _returnvalue))
    (else
      (for _array_element _disponiblespaces
        (Development|PrintString "---")
        (Development|PrintString (Utilities|String|ToString(Integer) _array_element))
        (return false "")))))

(fn CheckLSpace)

(fn PawnMovement
  ;[1 1 1] FrontAndBackTiles
  (MovementType|CheckFrontBackSpace (Variables|Default|GetReach) (.x (Variables|Default|GetTileSize)))
  (MovementType|CheckFrontBackSpace (Variables|Default|GetReach) (* (.x (Variables|Default|GetTileSize)) -1.0))
  ;[1 1 1] Left And Right Tiles
  (MovementType|CheckLeftRightSpaces (Variables|Default|GetReach) (.y (Variables|Default|GetTileSize)))
  (MovementType|CheckLeftRightSpaces (Variables|Default|GetReach) (* (.y (Variables|Default|GetTileSize)) -1.0)))

(fn PawnAttack
  ;[1 1 1] Front Diagonal Tiles
  (MovementType|CheckDiagonal+X (Variables|Default|GetReachDiag) (.y (Variables|Default|GetTileSize)))
  (MovementType|CheckDiagonal+X (Variables|Default|GetReachDiag) (* (.y (Variables|Default|GetTileSize)) -1.0))
  ;[1 1 1] Back Diagonal Tiles
  (MovementType|CheckDiagonal-X (Variables|Default|GetReachDiag) (.y (Variables|Default|GetTileSize)))
  (MovementType|CheckDiagonal-X (Variables|Default|GetReachDiag) (* (.y (Variables|Default|GetTileSize)) -1.0)))

(fn BishopMovement
  ;[1 1 1] Front Diagonal Tiles
  (MovementType|CheckDiagonal+X (+ (Variables|Default|GetReachDiag) 2) (.y (Variables|Default|GetTileSize)))
  (MovementType|CheckDiagonal+X (+ (Variables|Default|GetReachDiag) 2) (* (.y (Variables|Default|GetTileSize)) -1.0))
  ;[1 1 1] Back Diagonal Tiles
  (MovementType|CheckDiagonal-X (+ (Variables|Default|GetReachDiag) 2) (.y (Variables|Default|GetTileSize)))
  (MovementType|CheckDiagonal-X (+ (Variables|Default|GetReachDiag) 2) (* (.y (Variables|Default|GetTileSize)) -1.0)))

(fn RookMovement
  ;[1 1 1] FrontAndBackTiles
  (MovementType|CheckFrontBackSpace (+ (Variables|Default|GetReach) 4) (.x (Variables|Default|GetTileSize)))
  (MovementType|CheckFrontBackSpace (+ (Variables|Default|GetReach) 4) (* (.x (Variables|Default|GetTileSize)) -1.0))
  ;[1 1 1] Left And Right Tiles
  (MovementType|CheckLeftRightSpaces (+ (Variables|Default|GetReach) 4) (.y (Variables|Default|GetTileSize)))
  (MovementType|CheckLeftRightSpaces (+ (Variables|Default|GetReach) 4) (* (.y (Variables|Default|GetTileSize)) -1.0)))
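; Chess-style grid piece that takes mesh and collision box from its PieceType and snaps to BP_Grid on BeginPlay.
; ActivatePiece builds per-type offsets out to Reach, then drops same-side occupied and non-walkable tiles.
; PieceMove lerps along a timeline, destroys the overlapped adversary on finish, and locks movement until ResetTurn.
; Select and UnSelect set outline color and scale, but CreateOutline and DestroyOutline are empty, their logic disconnected.
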(event Custom|PieceMove
  (params (FinalPoint :type Vector))
  (bind _meshcomp (Variables|Default|GetMeshComp))
  ;[0 0 0] Gradualy Move the piece
  (if (Variables|Default|GetCanmove)
    (Variables|Movement|SetDestination FinalPoint)
    (Variables|Movement|SetStart (Transformation|GetActorLocation))
    (bind _alpha (Timeline|Timeline_1 PlayFromStart) ; Move Speed
      (:Update
        (Variables|Default|SetCanmove false)
        (Transformation|SetActorLocation (Math|Vector|Lerp(Vector) (Variables|Movement|GetStart) (Variables|Movement|GetDestination) _alpha) false false) ; Set Base Location
        (Utilities|IsValid _meshcomp
          (:Is%20Valid
            (Transformation|SetWorldLocation _meshcomp (Math|Vector|Lerp(Vector) (Variables|Movement|GetStart) (Variables|Movement|GetDestination) _alpha) false false))))
      (:Finished
        (Actor|DestroyActor (Collision|GetOverlappingActors (Variables|Default|GetBox) (Variables|Default|GetAdversarry) :!class /Script/Engine.PrimitiveComponent))))))

(event EventBeginPlay
  ;[0 0 0] Begin Play Set Variables
  (Utilities|FlowControl|Sequence
    (:then_0
      (bind _asbp_pawn (Utilities|Casting|CastToBP_Pawn (Game|Player|GetPlayerPawn 0)))
      (Variables|Default|SetPlayer _asbp_pawn)
      (Variables|Default|SetCanmove true))
    (:then_1
      (Variables|Outline|SetHasOutline false)
      (Variables|Default|SetAtualMesh (Variables|/Script/Engine.SkinnedMeshComponent|GetSkeletalMesh (Variables|Default|GetSkeletalMesh)))
      (bind _output_get (Variables|Outline|SetColor "(R=1.000000,G=1.000000,B=1.000000,A=1.000000)"))
      (Variables|Default|SetOGColor _output_get)
      (bind _output_get_2 (Variables|Outline|SetScale 1.0))
      (Variables|Default|SetOGScale _output_get_2)
      (bind _returnvalue (Actor|GetActorOfClass "/Game/Blueprints/Core/Grid/BP_Grid.BP_Grid_C"))
      (Variables|Default|SetGrid _returnvalue)
      ;;[1 1 1] Fix
      (Utilities|FlowControl|Delay 0.2)
      (CallFunction|SetBaseLocation)
      (CallFunction|CreateOutline))))

(fn ConstructionScript
  (bind _box (Variables|Default|GetBox))
  (bind _relativelocation (Variables|/Script/Engine.SceneComponent|GetRelativeLocation _box))
  (bind _unit_data (CallFunction|GetDefaultPieceDatafromType (Variables|Default|GetPieceType)))
  (Class|SkinnedMeshComponent|SetSkeletalMesh (Variables|Default|GetSkeletalMesh) (.skeletalmesh (Utilities|Struct|BreakS_PieceData _unit_data)) true)
  (Components|Box|SetBoxExtent (Variables|Default|GetBox) (.boxextend (Utilities|Struct|BreakS_PieceData _unit_data)) true)
  (Transformation|SetRelativeLocation _box (Math|Vector|MakeVector (.x _relativelocation) (.y _relativelocation) (.boxheight (Utilities|Struct|BreakS_PieceData _unit_data))) false false))

(fn CreateOutline)

(fn DestroyOutline)

(fn ClearSpaces
  (Utilities|Array|Clear (Variables|Default|GetDisponibleSpaces)))

(fn Select
  ;[0.6798 0.1602 1] Save Piece And Change Its Outline
  (Variables|Default|SetSelected true)
  (Variables|Outline|SetColor "(R=1.000000,G=0.887345,B=0.000000,A=1.000000)")
  (Variables|Outline|SetScale (* (Variables|Default|GetOGScale) 3.0))
  (CallFunction|DestroyOutline)
  (CallFunction|CreateOutline)
  (CallFunction|ClearSpaces))

(fn UnSelect
  (Variables|Default|SetSelected false)
  (Variables|Outline|SetColor (Variables|Default|GetOGColor))
  (Variables|Outline|SetScale (Variables|Default|GetOGScale))
  (CallFunction|DestroyOutline)
  (CallFunction|CreateOutline))

(fn CheckPieceLocation
  (bind _returnvalue (Transformation|GetActorLocation))
  (bind (_returnvalue_2 _index) (Default|CheckPieceLocation (Variables|Default|GetGrid) (+ _returnvalue "0, 0,1000.000000") (- _returnvalue "0, 0,1000.000000")))
  (return _returnvalue_2 _index))

(fn SetBaseLocation
  (bind _returnvalue (Transformation|GetActorLocation))
  ;[0.5168 0.09321 1] Snap Piece To Grid Center
  (bind (_returnvalue_2 _index) (Default|CheckPieceLocation (Variables|Default|GetGrid) (+ _returnvalue "0, 0,1000.000000") (- _returnvalue "0, 0,1000.000000")))
  (if _returnvalue_2
    (if (.ReturnValue (Utilities|Map|Find (Variables|/Game/Blueprints/Core/Grid/BP_Grid.BP_Grid_C|GetGridTiles (Variables|Default|GetGrid)) _index))
      (Transformation|SetActorLocation (.location (.Transform (Utilities|Struct|BreakS_TileData (.Value (Utilities|Map|Find (Variables|/Game/Blueprints/Core/Grid/BP_Grid.BP_Grid_C|GetGridTiles (Variables|Default|GetGrid)) _index))))) false false))))

(fn CheckMovableSpace
  (params (Index :type Int%20Point%20Structure))
  (bind _disponiblespaces (Variables|Default|GetDisponibleSpaces))
  (bind _returnvalue (Utilities|Array|FindItem _disponiblespaces Index))
  (if (!= _returnvalue -1)
    (return true (Utilities|Array|Get(acopy) (Variables|Default|GetDisponibleSpaces) _returnvalue))
    (else
      (for _array_element _disponiblespaces
        (Development|PrintString "---")
        (Development|PrintString (Utilities|String|ToString(Integer) _array_element))
        (return false "")))))

(fn ResetTurn
  (Variables|Default|SetCanmove true))

(fn KingQueenMovement
  (params (Index :type Int%20Point%20Structure))
  (for _index (range 0 (- (Variables|Default|GetReach) 1))
    (LocalVariables|SetLoopIndex _index)
    (Utilities|Array|AppendArray (LocalVariables|GetRet) (Utilities|Array|MakeArray (+ Index (Utilities|Struct|MakeIntPoint (+ (LocalVariables|GetLoopIndex) 1) 0)) (+ Index (Utilities|Struct|MakeIntPoint 0 (+ (LocalVariables|GetLoopIndex) 1))) (+ Index (Utilities|Struct|MakeIntPoint (* (+ (LocalVariables|GetLoopIndex) 1) -1) 0)) (+ Index (Utilities|Struct|MakeIntPoint 0 (* (+ (LocalVariables|GetLoopIndex) 1) -1)))))
    (Utilities|Array|AppendArray (LocalVariables|GetRet) (Utilities|Array|MakeArray (+ Index (Utilities|Struct|MakeIntPoint (+ (LocalVariables|GetLoopIndex) 1) (+ (LocalVariables|GetLoopIndex) 1))) (+ Index (Utilities|Struct|MakeIntPoint (* (+ (LocalVariables|GetLoopIndex) 1) -1) (+ (LocalVariables|GetLoopIndex) 1))) (+ Index (Utilities|Struct|MakeIntPoint (* (+ (LocalVariables|GetLoopIndex) 1) -1) (* (+ (LocalVariables|GetLoopIndex) 1) -1))) (+ Index (Utilities|Struct|MakeIntPoint (+ (LocalVariables|GetLoopIndex) 1) (* (+ (LocalVariables|GetLoopIndex) 1) -1))))))
  (return (LocalVariables|GetRet)))

(fn PawnMovement
  (params (Index :type Int%20Point%20Structure))
  (for _index (range 0 (- (Variables|Default|GetReach) 1))
    (LocalVariables|SetLoopIndex _index)
    (Utilities|Array|AppendArray (LocalVariables|GetRet) (Utilities|Array|MakeArray (+ Index (Utilities|Struct|MakeIntPoint (+ (LocalVariables|GetLoopIndex) 1) 0)) (+ Index (Utilities|Struct|MakeIntPoint 0 (+ (LocalVariables|GetLoopIndex) 1))) (+ Index (Utilities|Struct|MakeIntPoint (* (+ (LocalVariables|GetLoopIndex) 1) -1) 0)) (+ Index (Utilities|Struct|MakeIntPoint 0 (* (+ (LocalVariables|GetLoopIndex) 1) -1))))))
  (return (LocalVariables|GetRet)))

(fn BishopMovement
  (params (Index :type Int%20Point%20Structure))
  (for _index (range 0 (- (Variables|Default|GetReach) 1))
    (LocalVariables|SetLoopIndex _index)
    (Utilities|Array|AppendArray (LocalVariables|GetRet) (Utilities|Array|MakeArray (+ Index (Utilities|Struct|MakeIntPoint (+ (LocalVariables|GetLoopIndex) 1) (+ (LocalVariables|GetLoopIndex) 1))) (+ Index (Utilities|Struct|MakeIntPoint (* (+ (LocalVariables|GetLoopIndex) 1) -1) (+ (LocalVariables|GetLoopIndex) 1))) (+ Index (Utilities|Struct|MakeIntPoint (* (+ (LocalVariables|GetLoopIndex) 1) -1) (* (+ (LocalVariables|GetLoopIndex) 1) -1))) (+ Index (Utilities|Struct|MakeIntPoint (+ (LocalVariables|GetLoopIndex) 1) (* (+ (LocalVariables|GetLoopIndex) 1) -1))))))
  (return (LocalVariables|GetRet)))

(fn RookMovement
  (params (Index :type Int%20Point%20Structure))
  (for _index (range 0 (- (Variables|Default|GetReach) 1))
    (LocalVariables|SetLoopIndex _index)
    (Utilities|Array|AppendArray (LocalVariables|GetRet) (Utilities|Array|MakeArray (+ Index (Utilities|Struct|MakeIntPoint (+ (LocalVariables|GetLoopIndex) 1) 0)) (+ Index (Utilities|Struct|MakeIntPoint 0 (+ (LocalVariables|GetLoopIndex) 1))) (+ Index (Utilities|Struct|MakeIntPoint (* (+ (LocalVariables|GetLoopIndex) 1) -1) 0)) (+ Index (Utilities|Struct|MakeIntPoint 0 (* (+ (LocalVariables|GetLoopIndex) 1) -1))))))
  (return (LocalVariables|GetRet)))

(fn KnightMovement
  (params (Index :type Int%20Point%20Structure))
  (for _index (range 0 (- (Variables|Default|GetReach) 1))
    (LocalVariables|SetLoopIndex _index)
    (Utilities|Array|AppendArray (LocalVariables|GetRet) (Utilities|Array|MakeArray (+ Index (Utilities|Struct|MakeIntPoint (+ (LocalVariables|GetLoopIndex) 1) (+ (+ (LocalVariables|GetLoopIndex) 1) 1))) (+ Index (Utilities|Struct|MakeIntPoint (+ (LocalVariables|GetLoopIndex) 1) (- (* (+ (LocalVariables|GetLoopIndex) 1) -1) 1))) (+ Index (Utilities|Struct|MakeIntPoint (* (+ (LocalVariables|GetLoopIndex) 1) -1) (+ (+ (LocalVariables|GetLoopIndex) 1) 1))) (+ Index (Utilities|Struct|MakeIntPoint (* (+ (LocalVariables|GetLoopIndex) 1) -1) (- (* (+ (LocalVariables|GetLoopIndex) 1) -1) 1)))))
    (Utilities|Array|AppendArray (LocalVariables|GetRet) (Utilities|Array|MakeArray (+ Index (Utilities|Struct|MakeIntPoint (+ (+ (LocalVariables|GetLoopIndex) 1) 1) (+ (LocalVariables|GetLoopIndex) 1))) (+ Index (Utilities|Struct|MakeIntPoint (+ (+ (LocalVariables|GetLoopIndex) 1) 1) (* (+ (LocalVariables|GetLoopIndex) 1) -1))) (+ Index (Utilities|Struct|MakeIntPoint (- (* (+ (LocalVariables|GetLoopIndex) 1) -1) 1) (+ (LocalVariables|GetLoopIndex) 1))) (+ Index (Utilities|Struct|MakeIntPoint (- (* (+ (LocalVariables|GetLoopIndex) 1) -1) 1) (* (+ (LocalVariables|GetLoopIndex) 1) -1))))))
  (return (LocalVariables|GetRet)))

(fn GetValidTilesMovement
  (params (IndexArray :type Array%20of%20Int%20Point%20Structures) (IsPlayer :type Boolean))
  (if IsPlayer
    (bind _outactors (Actor|GetAllActorsOfClass "/Game/Blueprints/Core/Player/Pieces/BPC_PieceControllable.BPC_PieceControllable_C"))
    (for _array_element _outactors
      (bind (_found _index) (CallFunction|CheckPieceLocation _array_element))
      (if _found
        (Utilities|Array|RemoveItem IndexArray _index)))
    (else
      (bind _outactors_2 (Actor|GetAllActorsOfClass "/Game/Blueprints/Core/Player/Pieces/BP_PieceEnemy.BP_PieceEnemy_C"))
      (for _array_element_2 _outactors_2
        (bind _asbp_piece_enemy (Utilities|Casting|CastToBP_PieceEnemy _array_element_2))
        (bind (_found_2 _index_2) (CallFunction|CheckPieceLocation _asbp_piece_enemy))
        (if _found_2
          (Utilities|Array|RemoveItem IndexArray _index_2)))))
  (for _array_element_3 IndexArray
    (bind _output_get (LocalVariables|SetData (.Value (Utilities|Map|Find (Variables|/Game/Blueprints/Core/Grid/BP_Grid.BP_Grid_C|GetGridTiles (Variables|Default|GetGrid)) _array_element_3))))
    (if (Default|IsTileTypeWalkable (Variables|Default|GetGrid) (Utilities|Struct|BreakS_TileData _output_get))
      (if (<= 0.0 (.z (Variables|/Game/Blueprints/Core/Grid/BP_Grid.BP_Grid_C|GetGridTile%20Size (Variables|Default|GetGrid))))
        (Utilities|Array|Add (LocalVariables|GetRet) (Utilities|Struct|BreakS_TileData (LocalVariables|GetData))))))
  (return (LocalVariables|GetRet)))

(fn ActivatePiece
  (bind (_found _index) (CallFunction|CheckPieceLocation))
  (if _found
    (switch Utilities|FlowControl|Switch|SwitchonE_PieceType (Variables|Default|GetPieceType)
      (:NewEnumerator0
        (bind _walkablespaces (Movement|PawnMovement _index))
        (bind _validwalkable (Movement|GetValidTilesMovement _walkablespaces (Variables|Default|GetIsplayer)))
        (bind _output_get (Variables|Default|SetValidMovement _validwalkable))
        (return _output_get))
      (:NewEnumerator1
        (bind _walkablespaces_2 (Movement|KnightMovement _index))
        (bind _validwalkable_2 (Movement|GetValidTilesMovement _walkablespaces_2 (Variables|Default|GetIsplayer)))
        (bind _output_get_2 (Variables|Default|SetValidMovement _validwalkable_2))
        (return _output_get_2))
      (:NewEnumerator2
        (bind _walkablespaces_3 (Movement|BishopMovement _index))
        (bind _validwalkable_3 (Movement|GetValidTilesMovement _walkablespaces_3 (Variables|Default|GetIsplayer)))
        (bind _output_get_3 (Variables|Default|SetValidMovement _validwalkable_3))
        (return _output_get_3))
      (:NewEnumerator3
        (bind _walkablespaces_4 (Movement|RookMovement _index))
        (bind _validwalkable_4 (Movement|GetValidTilesMovement _walkablespaces_4 (Variables|Default|GetIsplayer)))
        (bind _output_get_4 (Variables|Default|SetValidMovement _validwalkable_4))
        (return _output_get_4))
      (:NewEnumerator4
        (bind _walkablespaces_5 (Movement|KingQueenMovement _index))
        (bind _validwalkable_5 (Movement|GetValidTilesMovement _walkablespaces_5 (Variables|Default|GetIsplayer)))
        (bind _output_get_5 (Variables|Default|SetValidMovement _validwalkable_5))
        (return _output_get_5)))))
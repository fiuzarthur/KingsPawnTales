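; Base Blueprint for a player-controllable chess piece, extending a parent class and caching the player's BP_Pawn on BeginPlay.
; ActivatePiece runs only if the piece is inactive: it clears the outline, sets a yellow color and larger scale, and flags it activated.
; It then sends the player pawn toward the piece by setting its desired location and movement speed.
; Move takes a location but is an empty stub here.
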(event EventBeginPlay
  (|CallParentFunction)
  (bind _asbp_pawn (Utilities|Casting|CastToBP_Pawn (Game|Player|GetPlayerPawn 0)))
  (Variables|Default|SetPlayer _asbp_pawn))

(event Collision|EventActorBeginOverlap
  (params (OtherActor :type Actor%20Object%20Reference)))

(event EventTick
  (params (DeltaSeconds :type Float%20%28single-precision%29)))

(fn ConstructionScript
  (|CallParentFunction))

(fn ActivatePiece
  (bind _player (Variables|Default|GetPlayer))
  (if (not (Variables|Default|GetActivated))
    (CallFunction|DestroyOutline)
    (Variables|Default|SetColor "(R=1.000000,G=0.892245,B=0.145770,A=1.000000)")
    (Variables|Default|SetScale 3.0)
    (Variables|Default|SetActivated true)
    (Variables|/Game/Blueprints/Core/Player/BP_Pawn.BP_Pawn_C|SetLocationDesired _player (Transformation|GetActorLocation))
    (Variables|/Game/Blueprints/Core/Player/BP_Pawn.BP_Pawn_C|SetLocationSpeed _player 1e+01)))

(fn Move
  (params (Location :type Vector)))
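; BP_Outline is a Blueprint that shows a static mesh with a colored outline, created on BeginPlay.
; CreateOutline spawns an unattached duplicate mesh at the original's world transform, using a dynamic M_OutlineClean_White instance on slot 0 driven by Color and Scale.
; DeleteOutline destroys that duplicate, with HasOutline preventing repeated creation.
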(event Custom|CreateOutline
  ;[0 0 0] Create Outliner
  (if (not (Variables|Default|GetHasOutline))
    (bind _returnvalue (AddComponent|AddStaticMeshComponent true (Transformation|GetWorldTransform (Variables|Default|GetStaticMesh))))
    (bind _output_get (Variables|Default|SetMeshComp _returnvalue))
    (Components|StaticMesh|SetStaticMesh _output_get (Variables|Default|GetNew%20Mesh))
    (bind _returnvalue_2 (Rendering|Material|CreateDynamicMaterialInstance (Variables|Default|GetMeshComp) 0 "/Game/Art/Materials/Outline/M_OutlineClean_White.M_OutlineClean_White" "None" :!class /Script/Engine.PrimitiveComponent))
    (Rendering|Material|SetVectorParameterValue _returnvalue_2 "color" (Variables|Default|GetColor) :!class /Script/Engine.MaterialInstanceDynamic)
    (Rendering|Material|SetScalarParameterValue _returnvalue_2 "Scale" (Variables|Default|GetScale) :!class /Script/Engine.MaterialInstanceDynamic)
    (Variables|Default|SetHasOutline true)))

(event Custom|DeleteOutline
  (bind _meshcomp (Variables|Default|GetMeshComp))
  ;[0 0 0] Delete Outliner
  (Utilities|IsValid _meshcomp
    (:Is%20Valid
      (Components|DestroyComponent _meshcomp)
      (Variables|Default|SetHasOutline false))))

(event EventBeginPlay
  ;[0 0 0] BeginPlay
  (Components|StaticMesh|SetStaticMesh (Variables|Default|GetStaticMesh) (Variables|Default|GetNew%20Mesh))
  (CallFunction|CreateOutline))

(fn ConstructionScript)